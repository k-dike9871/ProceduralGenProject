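; Double door Blueprint that opens when the player walks into its Overlap component while holding a key.
; On overlap it casts the player to ThirdPersonCharacter, then either spends one key and opens, or prints a "KEY NEEDED" message.
; A timeline lerps both doors from rotations saved at BeginPlay toward opposite half-turn targets.
; No opened state is tracked, so each overlap with keys available spends another.
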(event OnComponentBeginOverlap(Overlap)
  (params (OverlappedComponent :type Primitive%20Component%20Object%20Reference) (OtherActor :type Actor%20Object%20Reference) (OtherComp :type Primitive%20Component%20Object%20Reference) (OtherBodyIndex :type Integer) (bFromSweep :type Boolean) (SweepResult :type Hit%20Result%20Structure%20%28by%20ref%29))
  (if (== OtherActor (Game|GetPlayerCharacter 0)) ; Overlap With Player
    (bind _asthird_person_character (Utilities|Casting|CastToThirdPersonCharacter (Game|GetPlayerCharacter 0))) ; Get Player
    (bind _output_get (Variables|Default|SetChar%20REF _asthird_person_character))
    (if (> (Variables|/Game/ThirdPersonBP/Blueprints/ThirdPersonCharacter.ThirdPersonCharacter_C|GetKeys _output_get) 0) ; Does Player Have Key?
      (|TakeKey)
      (CallFunction|OpenDoors)
      (else
        (Development|PrintString "KEY NEEDED")))))

(event Custom|Open%20Doors
  (bind _0_to_1 (Timeline|0%20To%201 Play)
    (:Update
      (Transformation|SetRelativeRotation (Variables|Default|GetDoor1) (Math|Rotator|Lerp(Rotator) (Variables|Default|GetDoor%201%20Origin) "0,-180.000000, 0" _0_to_1 true) false false)
      (Transformation|SetRelativeRotation (Variables|Default|GetDoor2) (Math|Rotator|Lerp(Rotator) (Variables|Default|GetDoor%202%20Origin) "0,180.000000, 0" _0_to_1 true) false false))))

(event EventBeginPlay
  (Variables|Default|SetDoor%201%20Origin (Variables|/Script/Engine.SceneComponent|GetRelativeRotation (Variables|Default|GetDoor1)))
  (Variables|Default|SetDoor%202%20Origin (Variables|/Script/Engine.SceneComponent|GetRelativeRotation (Variables|Default|GetDoor2))))

(fn ConstructionScript)