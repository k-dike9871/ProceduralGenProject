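; Random level generator actor that builds a NumX by NumY grid of streamed level instances around itself on BeginPlay.
; Specific-level entries can pin their own level pool to a 1-based cell, or get random coordinates first; the first match wins.
; Other cells draw from the default LevelNames list.
; Each pick becomes a uniquely named streaming level instance, offset by LevelSize, randomly yawed in 90-degree steps and block-loaded visible.
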(event EventBeginPlay
  (CallFunction|CheckforEntriesThatNeedCoordinates)
  (for _index (range 0 (- (Variables|Default|GetNum%20X) 1))
    (Variables|Default|SetLoop%20X _index)
    (for _index_2 (range 0 (- (Variables|Default|GetNum%20Y) 1))
      (Variables|Default|SetLoop%20Y _index_2)
      (bind (_level_details1 _found_information1) (CallFunction|CheckforSpecifcLevelInfo))
      (if _found_information1
        (CallFunction|PickandSpawnLevelfromArray (.LevelNames (Utilities|Struct|BreakSpecificLevelInfo _level_details1)))
        (else
          (CallFunction|PickandSpawnLevelfromArray (Variables|Default|GetLevel%20Names)))))))

(fn ConstructionScript)

(fn PickandSpawnLevelfromArray
  (params (InputPin :type Array%20of%20Names))
  (bind _returnvalue (Class|LevelStreaming|CreateInstance (Class|GameplayStatics|GetStreamingLevel (Utilities|Array|Get(acopy) InputPin (Math|Random|RandomIntegerinRange 0 (Utilities|Array|LastIndex InputPin)))) (Utilities|String|Append (Utilities|String|ToString(Integer) (Variables|Default|GetLoop%20X)) "x" (Utilities|String|ToString(Integer) (Variables|Default|GetLoop%20Y)) (Utilities|GetDisplayName self)))) ; Each instance created needs a name
  (Variables|/Script/Engine.LevelStreaming|SetLevelTransform _returnvalue (Math|Transform|MakeTransform (+ (Math|Vector|MakeVector (- (* (Variables|Default|GetLoop%20X) (Variables|Default|GetLevel%20Size)) (/ (* (Variables|Default|GetNum%20X) (Variables|Default|GetLevel%20Size)) 2.0)) (+ (- (* (Variables|Default|GetLoop%20Y) (Variables|Default|GetLevel%20Size)) (/ (* (Variables|Default|GetNum%20Y) (Variables|Default|GetLevel%20Size)) 2.0)) (/ (Variables|Default|GetLevel%20Size) 2.0)) 0.0) (Transformation|GetActorLocation)) (Math|Rotator|MakeRotator 0.0 0.0 (* (Math|Random|RandomIntegerinRange 0 3) 9e+01))))
  (Variables|/Script/Engine.LevelStreaming|SetbShouldBlockOnLoad _returnvalue true)
  (Variables|/Script/Engine.LevelStreaming|SetbShouldBeLoaded _returnvalue true)
  (Variables|/Script/Engine.LevelStreaming|SetbShouldBeVisible _returnvalue true))

(fn CheckforSpecifcLevelInfo
  (LocalVariables|SetFound%20Information false)
  (for _array_element (Variables|Default|GetSpecifc%20Level%20Info)
    (if (not (LocalVariables|GetFound%20Information))
      (if (and (== (+ (Math|Float|Round (.X (Math|Vector|BreakVector (.Coordinates (Utilities|Struct|BreakSpecificLevelInfo _array_element))))) -1) (Variables|Default|GetLoop%20X)) (== (+ (Math|Float|Round (.Y (Math|Vector|BreakVector (.Coordinates (Utilities|Struct|BreakSpecificLevelInfo _array_element))))) -1) (Variables|Default|GetLoop%20Y)))
        (LocalVariables|SetLevel%20Details _array_element)
        (LocalVariables|SetFound%20Information true))))
  (return (LocalVariables|GetLevel%20Details) (LocalVariables|GetFound%20Information)))

(fn CheckforEntriesThatNeedCoordinates
  (for (_array_element _array_index) (Variables|Default|GetSpecifc%20Level%20Info)
    (if (.GetRandomCoordinatesOnStart? (Utilities|Struct|BreakSpecificLevelInfo _array_element))
      (Utilities|Array|SetArrayElem (Variables|Default|GetSpecifc%20Level%20Info) _array_index (Utilities|Struct|MakeSpecificLevelInfo (Math|Vector|MakeVector (Math|Conversions|ToFloat(Integer) (Math|Random|RandomIntegerinRange 1 (Variables|Default|GetNum%20X))) (Math|Conversions|ToFloat(Integer) (Math|Random|RandomIntegerinRange 1 (Variables|Default|GetNum%20Y))) 0.0) (.LevelNames (Utilities|Struct|BreakSpecificLevelInfo _array_element)) (.GetRandomCoordinatesOnStart? (Utilities|Struct|BreakSpecificLevelInfo _array_element))))))
  (return))