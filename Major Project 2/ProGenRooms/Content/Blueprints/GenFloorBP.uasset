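; GenFloorBP is an actor that builds a rectangular floor from repeated mesh pieces.
; Its construction script loops over X and Y counts, adding an instance to the Floor instanced mesh component at offsets spaced by mesh length and width.
; The grid is generated at construction, and the event graph holds only disabled placeholder events.
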(event EventBeginPlay)

(event Collision|EventActorBeginOverlap
  (params (OtherActor :type Actor%20Object%20Reference)))

(event EventTick
  (params (DeltaSeconds :type Float%20%28single-precision%29)))

(fn ConstructionScript
  (for _index (range 0 (- (Variables|Default|GetNumber%20Meshes%20X) 1)) ; X
    (for _index_2 (range 0 (- (Variables|Default|GetNumber%20Meshes%20Y) 1)) ; Y
      (Components|InstancedStaticMesh|AddInstance (Variables|Default|GetFloor) (Math|Transform|MakeTransform (Math|Vector|MakeVector (* _index (Variables|Default|GetMesh%20Length)) (* _index_2 (Variables|Default|GetMesh%20Width)) 0.0) "0, 0, 0" "1,1.000000,1")))))