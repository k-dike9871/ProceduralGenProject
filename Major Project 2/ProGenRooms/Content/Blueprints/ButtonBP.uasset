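; ButtonBP is an interactable button that opens the Door whose DoorValue matches its ButtonValue.
; On Interact, it searches all Door actors, opens the first match for the interacting Player and blends the first player controller's view to that door.
; Each non-matching door checked before a match applies damage to the first player character, so damage depends on search order and accumulates when none match.
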(event EventBeginPlay)

(event Collision|EventActorBeginOverlap
  (params (OtherActor :type Actor%20Object%20Reference)))

(event EventTick
  (params (DeltaSeconds :type Float%20%28single-precision%29)))

(event EventInteract
  (params (Player :type Character%20Object%20Reference))
  ;[1 1 1] Button Function
  (bind _outactors (Actor|GetAllActorsOfClass "/Game/Blueprints/Door.Door_C"))
  (bind _array_element (Utilities|Array|ForEachLoopwithBreak _outactors :!label _label)
    (:LoopBody
      (if (== (Variables|/Game/Blueprints/Door.Door_C|GetDoor%20Value _array_element) (Variables|Default|GetButton%20Value))
        (Default|OpenDoor _array_element Player)
        (Game|Player|SetViewTargetwithBlend (Game|GetPlayerController 0) _array_element 0.0 "VTBlend_Linear" 0.0 false)
        (goto _label Break)
        (else
          (Game|Damage|ApplyDamage (Game|GetPlayerCharacter 0) 1e+01 0 0))))))

(fn ConstructionScript)