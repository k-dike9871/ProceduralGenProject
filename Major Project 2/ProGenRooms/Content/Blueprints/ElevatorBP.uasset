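; Elevator platform Blueprint that rises while the player character stands in its trigger box and descends when they leave.
; Box overlap events play or reverse the Movement timeline, whose alpha lerps the static mesh's world location between the Move1 and Move2 markers.
; BeginPlay sets the timeline play rate from a Seconds variable to control travel duration.
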(event OnComponentBeginOverlap(Box)
  (params (OverlappedComponent :type Primitive%20Component%20Object%20Reference) (OtherActor :type Actor%20Object%20Reference) (OtherComp :type Primitive%20Component%20Object%20Reference) (OtherBodyIndex :type Integer) (bFromSweep :type Boolean) (SweepResult :type Hit%20Result%20Structure%20%28by%20ref%29))
  (if (== OtherActor (Game|GetPlayerCharacter 0))
    (CallFunction|ElevatorUp)))

(event OnComponentEndOverlap(Box)
  (params (OverlappedComponent :type Primitive%20Component%20Object%20Reference) (OtherActor :type Actor%20Object%20Reference) (OtherComp :type Primitive%20Component%20Object%20Reference) (OtherBodyIndex :type Integer))
  (if (== OtherActor (Game|GetPlayerCharacter 0))
    (CallFunction|ElevatorDown)))

(event Custom|Elevator%20Up
  (bind _0_to_1 (Timeline|Movement Play)
    (:Update
      (Transformation|SetWorldLocation (Variables|Default|GetStaticMesh) (Math|Vector|Lerp(Vector) (Transformation|GetWorldLocation (Variables|Default|GetMove%201)) (Transformation|GetWorldLocation (Variables|Default|GetMove%202)) _0_to_1) false false))))

(event Custom|Elevator%20Down
  (bind _0_to_1 (Timeline|Movement Reverse)
    (:Update
      (Transformation|SetWorldLocation (Variables|Default|GetStaticMesh) (Math|Vector|Lerp(Vector) (Transformation|GetWorldLocation (Variables|Default|GetMove%201)) (Transformation|GetWorldLocation (Variables|Default|GetMove%202)) _0_to_1) false false))))

(event EventBeginPlay
  (Components|Timeline|SetPlayRate (Variables|Default|GetMovement) (/ 1.0 (Variables|Default|Getseconds))))

(fn ConstructionScript)