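; Battery pickup actor that the player collects with the Interact input while standing inside its Box trigger.
; Box overlap by ThirdPersonCharacter shows an Interaction_Prompt_Widget and opens a gate, and leaving removes the prompt and closes it.
; Interact briefly flags the widget as pressed, then, if the gate is open, calls BatteryPickup on the character, plays a click sound and destroys the actor.
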(event OnComponentBeginOverlap(Box)
  (params (OverlappedComponent :type Primitive%20Component%20Object%20Reference) (OtherActor :type Actor%20Object%20Reference) (OtherComp :type Primitive%20Component%20Object%20Reference) (OtherBodyIndex :type Integer) (bFromSweep :type Boolean) (SweepResult :type Hit%20Result%20Structure%20%28by%20ref%29))
  (bind _asthird_person_character (Utilities|Casting|CastToThirdPersonCharacter OtherActor))
  (bind _returnvalue (UserInterface|CreateWidget "/Game/Widgets_UI/Interaction_Prompt_Widget.Interaction_Prompt_Widget_C"))
  (UserInterface|Viewport|AddtoViewport _returnvalue 0)
  (Utilities|FlowControl|Gate true) ; enters at Open
)

(event OnComponentEndOverlap(Box)
  (params (OverlappedComponent :type Primitive%20Component%20Object%20Reference) (OtherActor :type Actor%20Object%20Reference) (OtherComp :type Primitive%20Component%20Object%20Reference) (OtherBodyIndex :type Integer))
  (Utilities|Casting|CastToThirdPersonCharacter OtherActor)
  (Widget|RemovefromParent (stale OnComponentBeginOverlap(Box) _returnvalue))
  (Utilities|FlowControl|Gate true) ; enters at Close
)

(event OnComponentBeginOverlap(Sphere)
  (params (OverlappedComponent :type Primitive%20Component%20Object%20Reference) (OtherActor :type Actor%20Object%20Reference) (OtherComp :type Primitive%20Component%20Object%20Reference) (OtherBodyIndex :type Integer) (bFromSweep :type Boolean) (SweepResult :type Hit%20Result%20Structure%20%28by%20ref%29)))

(event OnComponentEndOverlap(Sphere)
  (params (OverlappedComponent :type Primitive%20Component%20Object%20Reference) (OtherActor :type Actor%20Object%20Reference) (OtherComp :type Primitive%20Component%20Object%20Reference) (OtherBodyIndex :type Integer)))

(event EventBeginPlay
  (Input|EnableInput (Game|GetPlayerController 0)))

(event Input|ActionEvents|InputActionInteract
  (params (Key :type Key%20Structure :default "None"))
  (:Pressed
    (Variables|/Game/Widgets_UI/Interaction_Prompt_Widget.Interaction_Prompt_Widget_C|SetIsPressed? (stale OnComponentBeginOverlap(Box) _returnvalue) true)
    (Utilities|FlowControl|Delay 0.2)
    (Variables|/Game/Widgets_UI/Interaction_Prompt_Widget.Interaction_Prompt_Widget_C|SetIsPressed? (stale OnComponentBeginOverlap(Box) _returnvalue) false)
    (Utilities|FlowControl|Gate true
      (:Exit
        (Default|BatteryPickup (stale OnComponentBeginOverlap(Box) _asthird_person_character))
        (Audio|PlaySoundatLocation "/Engine/VREditor/Sounds/UI/Click_on_Button_Cue.Click_on_Button_Cue" (Transformation|GetActorLocation) "0, 0, 0" 1.0 1.0 0.0 0 0 0)
        (Actor|DestroyActor)))))

(fn ConstructionScript)