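; Health pickup Blueprint that heals the player's third-person character on contact.
; When a ThirdPersonCharacter overlaps its Box, it checks the character's HealthBP and acts only if health is below maximum.
; Healing reuses the damage system by calling ApplyDamage with a negated HealAmount, then the pickup destroys itself and plays a 2D pickup sound.
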(event OnComponentBeginOverlap(Box)
  (params (OverlappedComponent :type Primitive%20Component%20Object%20Reference) (OtherActor :type Actor%20Object%20Reference) (OtherComp :type Primitive%20Component%20Object%20Reference) (OtherBodyIndex :type Integer) (bFromSweep :type Boolean) (SweepResult :type Hit%20Result%20Structure%20%28by%20ref%29))
  (bind _asthird_person_character (Utilities|Casting|CastToThirdPersonCharacter OtherActor))
  (if (< (Variables|/Game/Blueprints/HealthBP.HealthBP_C|GetHealth (Variables|/Game/ThirdPersonBP/Blueprints/ThirdPersonCharacter.ThirdPersonCharacter_C|GetHealthBP _asthird_person_character)) (Variables|/Game/Blueprints/HealthBP.HealthBP_C|GetMax%20Health (Variables|/Game/ThirdPersonBP/Blueprints/ThirdPersonCharacter.ThirdPersonCharacter_C|GetHealthBP _asthird_person_character)))
    (Game|Damage|ApplyDamage _asthird_person_character (* (Variables|Default|GetHeal%20Amount) -1.0) 0 0)
    (Actor|DestroyActor)
    (Audio|PlaySound2D "/Game/SFX/204318__juancamiloorjuela__pick-up-health__1_.204318__juancamiloorjuela__pick-up-health__1_" 1.0 1.0 0.0 0 0)))

(event EventBeginPlay)

(event Collision|EventActorBeginOverlap
  (params (OtherActor :type Actor%20Object%20Reference)))

(event EventTick
  (params (DeltaSeconds :type Float%20%28single-precision%29)))

(fn ConstructionScript)